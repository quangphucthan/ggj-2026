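; BP_Object is a block that is visible and solid only while the player's mask is on.
; It starts hidden without collision, set by the construction script and again at BeginPlay regardless of the current mask state.
; BeginPlay binds HandleMaskToggle to BP_Baymax_Character's mask-state event.
; Each change feeds UpdateMaskVisuals, which switches the Cube's visibility and collision together.
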(event `self.ReceiveBeginPlay`
  ; Make the block disappear after pressing "E"
  (bind _asbp_baymax_character (cast `/Game/Characters/Baymax/SkeletalMeshes/Blueprinta/BP_Baymax_Character` (`GameplayStatics.GetPlayerCharacter` 0)))
  (add `/Game/Characters/Baymax/SkeletalMeshes/Blueprinta/BP_Baymax_Character.OnMaskStateChanged` _asbp_baymax_character (delegate `HandleMaskToggle`))
  (if (`/Game/Characters/Baymax/SkeletalMeshes/Blueprinta/BP_Baymax_Character.bIsMaskEquipped` _asbp_baymax_character)
    _
    (else
      _))
  (`self.UpdateMaskVisuals` false))

(event `HandleMaskToggle`
  (params (NewState :type Boolean))
  ; Make the block disappear after pressing "E"
  (`self.UpdateMaskVisuals` NewState))

(fn `UpdateMaskVisuals`
  (params (Condition :type Boolean))
  (bind _cube (`self.Cube`))
  ; Update visual and physics based on the boolean variables
  (if Condition
    (`SceneComponent.SetVisibility` _cube true false)
    (`PrimitiveComponent.SetCollisionEnabled` _cube "QueryAndPhysics")
    (else
      (`SceneComponent.SetVisibility` _cube false false)
      (`PrimitiveComponent.SetCollisionEnabled` _cube "NoCollision"))))

(fn `UserConstructionScript`
  (bind _cube (`self.Cube`))
  (`SceneComponent.SetVisibility` _cube false false)
  (`PrimitiveComponent.SetCollisionEnabled` _cube "NoCollision"))